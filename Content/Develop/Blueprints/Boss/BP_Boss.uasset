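; BP_Boss is a boss actor that starts with a fixed health value and provides an attack event.
; The Attack event rotates the boss toward an actor found by GetActorOfClass.
; It then briefly sets the Attack flag on the ABP_Boss animation instance, clearing it after a short delay.
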(event Custom|Attack
  (bind _returnvalue (Actor|GetActorOfClass 0))
  (Transformation|SetActorRotation (Math|Rotator|FindLookatRotation (Transformation|GetActorLocation) (Transformation|GetActorLocation _returnvalue)))
  (bind _asabp_boss (Utilities|Casting|CastToABP_Boss (Components|SkeletalMesh|GetAnimInstance (Variables|Character|GetMesh))))
  (Variables|/Game/Develop/Blueprints/Boss/ABP_Boss.ABP_Boss_C|SetAttack _asabp_boss true)
  (Utilities|FlowControl|Delay 0.5)
  (Variables|/Game/Develop/Blueprints/Boss/ABP_Boss.ABP_Boss_C|SetAttack _asabp_boss false))

(event EventBeginPlay
  (Variables|Default|SetHp 5e+02))

(fn ConstructionScript)